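; BP_Slime is a slime enemy character that hops repeatedly on a looping one-second timer.
; When the timer fires, it jumps if its vertical velocity is zero, otherwise it stores the jump.
; On landing with a stored jump, it clears the timer, waits a tick, jumps and restarts the timer so the rhythm follows the landing.
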(event `self.ReceiveBeginPlay`
  ;[0.1827 1 0.152] The slime enemy will jump every second
  (bind _returnvalue (`KismetSystemLibrary.K2_SetTimerDelegate` (delegate `EnemyJump`) 1.0 true :!label _label))
  (set `self.JumpTimer` _returnvalue))

(event `EnemyJump`
  (bind (_returnvalue_x _returnvalue_y _returnvalue_z) (`KismetMathLibrary.BreakVector` (`self.GetVelocity`)))
  ;[0.1827 1 0.152] The slime enemy will jump every second
  (if (== _returnvalue_z 0.0)
    (`self.Jump`)
    (else
      (set `self.storedJump?` true))))

(event `self.OnLanded`
  (params (Hit :type "HitResult Structure (by ref)"))
  ;[0.1827 1 0.152] The slime enemy will jump every second
  (if (`self.storedJump?`)
    (`KismetSystemLibrary.K2_ClearAndInvalidateTimerHandle` (`self.JumpTimer`))
    (set `self.storedJump?` false)
    (`KismetSystemLibrary.DelayUntilNextTick`)
    (`self.Jump`)
    (goto _label)))

(fn `UserConstructionScript`
  (`parent.UserConstructionScript`))