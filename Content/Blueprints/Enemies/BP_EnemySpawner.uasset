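; BP_EnemySpawner is a placeable spawn point that creates one enemy of a chosen EnemyType: slime, shooter or big guy.
; Its construction script sets a preview sprite matching that type.
; When Spawn is called, it spawns the matching enemy Blueprint at the sprite's location with a fixed rotation, adjusting for collisions but always spawning, then destroys itself.
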(event `Spawn`
  (bind _returnvalue_location (`KismetMathLibrary.BreakTransform` (`SceneComponent.K2_GetComponentToWorld` (`self.PreviewSprite`))))
  (switch `/Game/Blueprints/Enemies/Enum_EnemyTypes` (`self.EnemyType`)
    (:`NewEnumerator0`
      (`|SpawnActorFromClass` "/Game/Blueprints/Enemies/BP_Slime.BP_Slime_C" (`KismetMathLibrary.MakeTransform` _returnvalue_location (struct :`Yaw` 180.0)) "AdjustIfPossibleButAlwaysSpawn" "MultiplyWithRoot" null null))
    (:`NewEnumerator1`
      (`|SpawnActorFromClass` "/Game/Blueprints/Enemies/BP_ShooterEnemy.BP_ShooterEnemy_C" (`KismetMathLibrary.MakeTransform` _returnvalue_location (struct :`Yaw` 180.0)) "AdjustIfPossibleButAlwaysSpawn" "MultiplyWithRoot" null null))
    (:`NewEnumerator2`
      (`|SpawnActorFromClass` "/Game/Blueprints/Enemies/BP_BigGuy.BP_BigGuy_C" (`KismetMathLibrary.MakeTransform` _returnvalue_location (struct :`Yaw` 180.0)) "AdjustIfPossibleButAlwaysSpawn" "MultiplyWithRoot" null null)))
  (`self.K2_DestroyActor`))

(fn `UserConstructionScript`
  (bind _previewsprite (`self.PreviewSprite`))
  (switch `/Game/Blueprints/Enemies/Enum_EnemyTypes` (`self.EnemyType`)
    (:`NewEnumerator0`
      (`PaperSpriteComponent.SetSprite` _previewsprite "/Game/Assets/Sprites/Enemy/tealSlime_0.tealSlime_0"))
    (:`NewEnumerator1`
      (`PaperSpriteComponent.SetSprite` _previewsprite "/Game/Assets/Sprites/Enemy/fireEnemy_0.fireEnemy_0"))
    (:`NewEnumerator2`
      (`PaperSpriteComponent.SetSprite` _previewsprite "/Game/Assets/Sprites/Player/protagonist_Idle_1_d.protagonist_Idle_1_d"))))