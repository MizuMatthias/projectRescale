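; BP_EnemyParent is a parent enemy Blueprint that patrols by constantly moving along its sprite's forward vector each tick.
; Wall detection begin-overlap and ledge detection end-overlap both call ChangeDirection, which turns the actor around with a 180-degree rotation.
; Capsule overlap with BP_playerCharacter only prints an "ENEMY DAMAGE" message; no damage is applied.
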(event `self.CapsuleComponent.OnComponentBeginOverlap`
  (params (OverlappedComponent :type "PrimitiveComponent Object Reference") (OtherActor :type "Actor Object Reference") (OtherComp :type "PrimitiveComponent Object Reference") (OtherBodyIndex :type Integer) (bFromSweep :type Boolean) (SweepResult :type "HitResult Structure (by ref)"))
  ;[1 1 1] Player contact damage
  (cast `/Game/Blueprints/Player/BP_playerCharacter` OtherActor)
  (`KismetSystemLibrary.PrintString` "ENEMY DAMAGE"))

(event `self.ReceiveTick`
  (params (DeltaSeconds :type "Float (single-precision)"))
  ;[1 1 1] Constant Movement
  (`self.AddMovementInput` (`SceneComponent.GetForwardVector` (`self.Sprite`))))

(event `self.WallDetection.OnComponentBeginOverlap`
  (params (OverlappedComponent :type "PrimitiveComponent Object Reference") (OtherActor :type "Actor Object Reference") (OtherComp :type "PrimitiveComponent Object Reference") (OtherBodyIndex :type Integer) (bFromSweep :type Boolean) (SweepResult :type "HitResult Structure (by ref)"))
  ;[1 1 1] Change direction at wall or ledge
  (`self.ChangeDirection`))

(event `self.LedgeDetection.OnComponentEndOverlap`
  (params (OverlappedComponent :type "PrimitiveComponent Object Reference") (OtherActor :type "Actor Object Reference") (OtherComp :type "PrimitiveComponent Object Reference") (OtherBodyIndex :type Integer))
  ;[1 1 1] Change direction at wall or ledge
  (`self.ChangeDirection`))

(fn `ChangeDirection`
  ;[1 1 1] Rotate Actor
  (`self.K2_SetActorRotation` (`KismetMathLibrary.ComposeRotators` (`self.K2_GetActorRotation`) (struct :`Yaw` 180.0))))

(fn `UserConstructionScript`)