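; Enemy fireball actor that damages the player on contact and destroys itself.
; A Hitbox overlap with BP_playerCharacter calls its placeholder ReduceHP, destroys the fireball and plays a hit sound.
; Any actor overlap also destroys it, logged as a wall collision.
; BeginPlay plays the firing sound and starts a timer that fizzles it out after a few seconds, with debug prints for each outcome.
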(event `self.ReceiveActorBeginOverlap`
  (params (OtherActor :type "Actor Object Reference"))
  (`KismetSystemLibrary.PrintString` "Fireball Collided With Wall and Destroyed" true true (struct :`R` 0.182707 :`G` 1.0 :`B` 0.151953 :`A` 1.0))
  (`self.K2_DestroyActor`))

(event `self.Hitbox.OnComponentBeginOverlap`
  (params (OverlappedComponent :type "PrimitiveComponent Object Reference") (OtherActor :type "Actor Object Reference") (OtherComp :type "PrimitiveComponent Object Reference") (OtherBodyIndex :type Integer) (bFromSweep :type Boolean) (SweepResult :type "HitResult Structure (by ref)"))
  (bind _asbp_player_character (cast `/Game/Blueprints/Player/BP_playerCharacter` OtherActor))
  ;[0.1827 1 0.152] Placeholder action - add health stuff when Matthew finishes it i guess idk
  (`/Game/Blueprints/Player/BP_playerCharacter.ReduceHP` _asbp_player_character)
  (`self.K2_DestroyActor`)
  (`GameplayStatics.PlaySound2D` "/Game/Blueprints/Sounds/enemy-hit_Cue.enemy-hit_Cue" 1.0 1.0 0.0 null null)
  (`KismetSystemLibrary.PrintString` "Fireball Hit Player and Destroyed Both" true true (struct :`R` 0.182707 :`G` 1.0 :`B` 0.151953 :`A` 1.0)))

(event `self.ReceiveBeginPlay`
  ;[0.1827 1 0.152] If fireball has not hit anything in 5 seconds, fizzle out and destroy fireball
  (`GameplayStatics.PlaySound2D` "/Game/Blueprints/Sounds/enemy-fireball_Cue.enemy-fireball_Cue" 1.0 1.0 0.0 null null)
  (`KismetSystemLibrary.K2_SetTimerDelegate` (delegate `Auto Delete`) 5.0))

(event `Auto Delete`
  ;[0.1827 1 0.152] If fireball has not hit anything in 5 seconds, fizzle out and destroy fireball
  (`self.K2_DestroyActor`)
  (`KismetSystemLibrary.PrintString` "Fireball Fizzled Out and Destroyed" true true (struct :`R` 0.182707 :`G` 1.0 :`B` 0.151953 :`A` 1.0)))

(fn `UserConstructionScript`)