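; BP_AimLine draws an aim trail from repeated crosshair trail sprites.
; AimStart caches a reference to the player character.
; Aim then adds scaled instances to a grouped sprite component at fixed steps along X, with the count set by DotCount.
; Each instance takes the camera's world rotation, while its position ignores camera direction, and existing instances are never cleared here.
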(event `AimStart`
  (bind _asbp_player_character (cast `/Game/Blueprints/Player/BP_playerCharacter` (`GameplayStatics.GetPlayerCharacter` 0)))
  (set `self.playerChar_REF` _asbp_player_character))

(event `Aim`
  (params (dotCount :type Integer))
  (for _index (range (+ dotCount 1))
    (`PaperGroupedSpriteComponent.AddInstance` (`self.PaperGroupedSprite`) (`KismetMathLibrary.MakeTransform` (`KismetMathLibrary.MakeVector` (`KismetMathLibrary.Conv_IntToDouble` (* _index 200))) (`SceneComponent.K2_GetComponentRotation` (`/Game/Blueprints/Player/BP_playerCharacter.Camera` (`self.playerChar_REF`))) (8.0 8.0 8.0)) "/Game/Assets/Sprites/UI/Aim/crosshairTrail_Sprite.crosshairTrail_Sprite" false (struct :`R` 1.0 :`G` 1.0 :`B` 1.0 :`A` 1.0))))

(fn `UserConstructionScript`)