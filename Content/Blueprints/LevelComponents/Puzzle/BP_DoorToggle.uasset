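; BP_DoorToggle is a puzzle level component for a door that slides vertically.
; Activate reverses the DoorMovement timeline if IsOpen is true and plays it otherwise, while Deactivate always reverses it.
; Timeline updates set the Cube's world Z to the root's height plus the track value scaled by TargetOffest, keeping the root's X and Y.
; IsOpen is only read in these graphs, never set.
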(event `self.Activate`
  (bind (_returnvalue_x _returnvalue_y _returnvalue_z) (`KismetMathLibrary.BreakVector` (`SceneComponent.K2_GetComponentLocation` (`self.DefaultSceneRoot`))))
  ;[1 1 1] When activated, move downwards/upwards by (x) units
  (if (`self.isOpen?`)
    (bind (_direction _newtrack_0) (`Timeline|DoorMovement` :!via `Reverse` :!label _label)
      (:`Update`
        (`SceneComponent.K2_SetWorldLocation` (`self.Cube`) (`KismetMathLibrary.MakeVector` _returnvalue_x _returnvalue_y (+ (* _newtrack_0 (`self.TargetOffest`)) _returnvalue_z)) false false)))
    (else
      (goto _label))))

(event `self.Deactivate`
  ;[1 1 1] When activated, move downwards/upwards by (x) units
  (goto _label :!via `Reverse`))

(fn `UserConstructionScript`
  (`parent.UserConstructionScript`))