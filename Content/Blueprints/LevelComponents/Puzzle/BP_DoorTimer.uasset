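; BP_DoorTimer is a timed puzzle door that moves vertically when activated, stays displaced for OpenTime, then returns.
; Activate ignores calls while IsActive is set, then plays the DoorMovement timeline, which sets the Cube's world Z from the root by TargetOffest.
; A FlipFlop on the timeline's Finished pin alternates between delaying then reversing, and clearing IsActive once the door is back.
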(event `self.Activate`
  (bind (_returnvalue_x _returnvalue_y _returnvalue_z) (`KismetMathLibrary.BreakVector` (`SceneComponent.K2_GetComponentLocation` (`self.DefaultSceneRoot`))))
  ;[1 1 1] When activated, move downwards/upwards by (x) units
  (if (not (`self.isActive?`))
    (set `self.isActive?` true)
    (bind (_direction _newtrack_0) (`Timeline|DoorMovement` :!label _label)
      (:`Update`
        (`SceneComponent.K2_SetWorldLocation` (`self.Cube`) (`KismetMathLibrary.MakeVector` _returnvalue_x _returnvalue_y (+ (* _newtrack_0 (`self.TargetOffest`)) _returnvalue_z)) false false))
      (:`Finished`
        (`/Engine/EditorBlueprintResources/StandardMacros.FlipFlop`
          (:`A`
            (`KismetSystemLibrary.Delay` (`self.OpenTime`))
            (goto _label :!via `Reverse`))
          (:`B`
            (set `self.isActive?` false)))))))

(fn `UserConstructionScript`
  (`parent.UserConstructionScript`))