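; BP_VerticalPushBlock is a puzzle block that BP_playerCharacter pushes up or down when its CurrentScale meets ScaleRequired.
; Two overlap boxes each trigger one direction, guarded by that direction's moving flag and a short Visibility trace for obstructions.
; A clear trace plays a timeline that offsets the block vertically from its start location without sweeping.
; Only the upward trace ignores BP_PushBlock actors, gathered at BeginPlay.
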(event `self.ReceiveBeginPlay`
  (bind _outactors (`GameplayStatics.GetAllActorsOfClass` "/Game/Blueprints/LevelComponents/Puzzle/BP_PushBlock.BP_PushBlock_C"))
  (set `self.Out Actors` _outactors))

(event `self.Box.OnComponentBeginOverlap`
  (params (OverlappedComponent :type "PrimitiveComponent Object Reference") (OtherActor :type "Actor Object Reference") (OtherComp :type "PrimitiveComponent Object Reference") (OtherBodyIndex :type Integer) (bFromSweep :type Boolean) (SweepResult :type "HitResult Structure (by ref)"))
  (bind _asbp_player_character (cast `/Game/Blueprints/Player/BP_playerCharacter` OtherActor))
  (if (and (>= (`/Game/Blueprints/Player/BP_playerCharacter.CurrentScale` _asbp_player_character) (`self.ScaleRequired`)) (not (`self.MovingDown?`)))
    (bind _output_get (set `self.StartLocation` (`self.K2_GetActorLocation`)))
    (bind (_outhit _returnvalue) (`KismetSystemLibrary.LineTraceSingle` _output_get (+ _output_get (0.0 0.0 -99.0)) "TraceTypeQuery1"))
    (if (not _returnvalue)
      (set `self.MovingDown?` true)
      (bind (_direction _movement) (`Timeline|DownwardsMovement` :!via `PlayFromStart`)
        (:`Update`
          (`self.K2_SetActorLocation` (+ (`self.StartLocation`) (`KismetMathLibrary.MakeVector` 0.0 0.0 _movement))))
        (:`Finished`
          (set `self.MovingUp?` false)
          (set `self.MovingDown?` false))))))

(event `self.Box1.OnComponentBeginOverlap`
  (params (OverlappedComponent :type "PrimitiveComponent Object Reference") (OtherActor :type "Actor Object Reference") (OtherComp :type "PrimitiveComponent Object Reference") (OtherBodyIndex :type Integer) (bFromSweep :type Boolean) (SweepResult :type "HitResult Structure (by ref)"))
  (bind _asbp_player_character (cast `/Game/Blueprints/Player/BP_playerCharacter` OtherActor))
  (if (and (>= (`/Game/Blueprints/Player/BP_playerCharacter.CurrentScale` _asbp_player_character) (`self.ScaleRequired`)) (not (`self.MovingUp?`)))
    (bind _output_get (set `self.StartLocation` (`self.K2_GetActorLocation`)))
    (bind (_outhit _returnvalue) (`KismetSystemLibrary.LineTraceSingle` _output_get (+ _output_get (0.0 0.0 99.0)) "TraceTypeQuery1" false (`self.Out Actors`)))
    (if (not _returnvalue)
      (set `self.MovingUp?` true)
      (bind (_direction _movement) (`Timeline|UpwardsMovement` :!via `PlayFromStart`)
        (:`Update`
          (`self.K2_SetActorLocation` (+ (`self.StartLocation`) (`KismetMathLibrary.MakeVector` 0.0 0.0 _movement))))
        (:`Finished`
          (set `self.MovingUp?` false)
          (set `self.MovingDown?` false))))))

(fn `UserConstructionScript`)