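; BP_WeightedPressurePlate is a puzzle pressure plate that switches linked level components on while the player stands on it.
; It caches the player character on BeginPlay, and its Box overlap events respond only to that actor.
; Entering the box calls Activate on each BP_ComponentParent in ComponentsToActivate, playing a switch sound per component.
; Leaving calls Deactivate on each, without sound.
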(event `self.ReceiveBeginPlay`
  (bind _asbp_player_character (cast `/Game/Blueprints/Player/BP_playerCharacter` (`GameplayStatics.GetPlayerCharacter` 0)))
  (set `self.Player REF` _asbp_player_character))

(event `self.Box.OnComponentBeginOverlap`
  (params (OverlappedComponent :type "PrimitiveComponent Object Reference") (OtherActor :type "Actor Object Reference") (OtherComp :type "PrimitiveComponent Object Reference") (OtherBodyIndex :type Integer) (bFromSweep :type Boolean) (SweepResult :type "HitResult Structure (by ref)"))
  (if (== OtherActor (`self.Player REF`))
    (for _array_element (`self.componentsToActivate`)
      (bind _asbp_component_parent (cast `/Game/Blueprints/LevelComponents/Puzzle/BP_ComponentParent` _array_element))
      (`/Game/Blueprints/LevelComponents/Puzzle/BP_ComponentParent.Activate` _asbp_component_parent)
      (`GameplayStatics.PlaySound2D` "/Game/Blueprints/Sounds/switch-activate_Cue.switch-activate_Cue" 1.0 1.0 0.0 null null))))

(event `self.Box.OnComponentEndOverlap`
  (params (OverlappedComponent :type "PrimitiveComponent Object Reference") (OtherActor :type "Actor Object Reference") (OtherComp :type "PrimitiveComponent Object Reference") (OtherBodyIndex :type Integer))
  (if (== OtherActor (`self.Player REF`))
    (for _array_element (`self.componentsToActivate`)
      (bind _asbp_component_parent (cast `/Game/Blueprints/LevelComponents/Puzzle/BP_ComponentParent` _array_element))
      (`/Game/Blueprints/LevelComponents/Puzzle/BP_ComponentParent.Deactivate` _asbp_component_parent))))

(fn `UserConstructionScript`)