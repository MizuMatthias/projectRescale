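; BP_DartTrap is a puzzle level component that fires an arrow when activated.
; Its Activate event spawns a BP_Arrow at the Cube component's world transform, ignoring collisions, then prints a placeholder debug string.
; It has no trigger logic of its own, as BeginPlay, overlap and Tick are disabled stubs and the construction script only calls its parent.
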(event `self.Activate`
  (`|SpawnActorFromClass` "/Game/Blueprints/Player/BP_Arrow.BP_Arrow_C" (`SceneComponent.K2_GetComponentToWorld` (`self.Cube`)) "AlwaysSpawn" "MultiplyWithRoot" null null)
  (`KismetSystemLibrary.PrintString` "Hello"))

(fn `UserConstructionScript`
  (`parent.UserConstructionScript`))