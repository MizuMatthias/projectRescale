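; Game Instance Blueprint that stores level completion progress across the game.
; An UpdateProgress event takes a level name and sets the matching completion flag to true.
; Five hard-coded name checks cover Level0 through Level4, each with its own boolean, and nothing here clears or saves them.
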(event `UpdateProgress`
  (params (LevelName :type String))
  (if (`KismetStringLibrary.EqualEqual_StrStr` LevelName "Level0")
    (set `self.completeLevel0?` true))
  (if (`KismetStringLibrary.EqualEqual_StrStr` LevelName "Level1")
    (set `self.completeLevel1?` true))
  (if (`KismetStringLibrary.EqualEqual_StrStr` LevelName "Level2")
    (set `self.completeLevel2?` true))
  (if (`KismetStringLibrary.EqualEqual_StrStr` LevelName "Level3")
    (set `self.completeLevel3?` true))
  (if (`KismetStringLibrary.EqualEqual_StrStr` LevelName "Level4")
    (set `self.completeLevel4?` true)))