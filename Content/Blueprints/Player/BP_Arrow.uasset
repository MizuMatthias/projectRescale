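; BP_Arrow is a projectile arrow that kills enemies it touches and becomes a pickup when it hits something solid.
; Projectile movement starts without gravity, then restores it after a short delay so the arrow flies flat at first.
; Overlapping a BP_EnemyParent destroys both the enemy and the arrow.
; A blocking hit stops movement and, a tick later, replaces the arrow with an ArrowPickup at its transform.
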(event `self.Sphere.OnComponentHit`
  (params (HitComponent :type "PrimitiveComponent Object Reference") (OtherActor :type "Actor Object Reference") (OtherComp :type "PrimitiveComponent Object Reference") (NormalImpulse :type "Vector Structure") (Hit :type "HitResult Structure (by ref)"))
  ;[1 1 1] Stop and spawn arrow pickup on hit
  (`ActorComponent.Deactivate` (`self.ProjectileMovement`))
  (`KismetSystemLibrary.DelayUntilNextTick`)
  (`|SpawnActorFromClass` "/Game/Blueprints/LevelComponents/Pickup/ArrowPickup.ArrowPickup_C" (`self.GetTransform`) "Undefined" "MultiplyWithRoot" null null)
  (`self.K2_DestroyActor`))

(event `self.Sphere.OnComponentBeginOverlap`
  (params (OverlappedComponent :type "PrimitiveComponent Object Reference") (OtherActor :type "Actor Object Reference") (OtherComp :type "PrimitiveComponent Object Reference") (OtherBodyIndex :type Integer) (bFromSweep :type Boolean) (SweepResult :type "HitResult Structure (by ref)"))
  ;[1 1 1] Destroy enemy and self on contact
  (bind _asbp_enemy_parent (cast `/Game/Blueprints/Enemies/BP_EnemyParent` OtherActor))
  (`self.K2_DestroyActor` _asbp_enemy_parent)
  (`self.K2_DestroyActor`))

(event `self.ProjectileMovement.OnComponentActivated`
  (params (Component :type "ActorComponent Object Reference") (bReset :type Boolean))
  ;[1 1 1] No gravity for 0.33s (about 400cm)
  (`KismetSystemLibrary.Delay` 0.333333)
  (set `ProjectileMovementComponent.ProjectileGravityScale` 1.0 (`self.ProjectileMovement`)))

(fn `UserConstructionScript`)